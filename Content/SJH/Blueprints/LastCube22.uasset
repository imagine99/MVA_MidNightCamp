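; LastCube22 is an actor that runs a short timed startup sequence and can hand off to the UI_Map level.
; One second after BeginPlay it zeroes the "cube" material parameter on its Cube, shows a loading screen and spawns a Cube actor at a fixed location.
; Pressing F sets the Next flag and prints a debug string.
; Next is checked only once, right after the spawn, so later presses do not open UI_Map.
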(event EventBeginPlay
  (Utilities|FlowControl|Delay 1.0)
  (Rendering|Material|SetScalarParameterValueonMaterials (Variables|Default|GetCube) "cube" 0.0)
  (Class|XRLoadingScreenFunctionLibrary|ShowLoadingScreen)
  (Game|SpawnActorfromClass "/Game/SJH/Blueprints/cube.cube_C" (Math|Transform|MakeTransform "-60.000000,-130.000000,160.000000" "0, 0, 0" "1.000000,1.000000,1.000000") "DontSpawnIfColliding" "MultiplyWithRoot" 0 0)
  (if (Variables|Default|Getnext)
    (Game|OpenLevel(byObjectReference) "/Game/SJH/Map/UI_Map.UI_Map")))

(event Input|KeyboardEvents|F
  (params (Key :type Key%20Structure :default "None"))
  (:Pressed
    (Variables|Default|Setnext true)
    (Development|PrintString "ffffff")))

(fn ConstructionScript)