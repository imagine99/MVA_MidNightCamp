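; BP_AI is a prototype AI pawn that works with Cook actors.
; Pressing Z spawns a half-scale Cook at a fixed location and sends the pawn toward a random reachable point via AI MoveTo.
; Any Box overlap waits 2.5 seconds, destroys all Cook actors and sets a flag.
; A SerchAround wander loop and random box scaling are left unconnected, with empty BeginPlay and Tick.
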(event OnComponentBeginOverlap(Box)
  (params (OverlappedComponent :type Primitive%20Component%20Object%20Reference) (OtherActor :type Actor%20Object%20Reference) (OtherComp :type Primitive%20Component%20Object%20Reference) (OtherBodyIndex :type Integer) (bFromSweep :type Boolean) (SweepResult :type Hit%20Result%20Structure%20%28by%20ref%29))
  (Utilities|FlowControl|Delay 2.5)
  (bind _outactors (Actor|GetAllActorsOfClass "/Game/LKH/My/My_BP/Eat/Cook.Cook_C"))
  (Actor|DestroyActor _outactors)
  (Variables|Default|SetNewVar true))

(event Custom|Serch%20Around)

(event EventBeginPlay)

(event EventTick
  (params (DeltaSeconds :type Float%20%28single-precision%29)))

(event Input|KeyboardEvents|Z
  (params (Key :type Key%20Structure))
  (:Pressed
    (Game|SpawnActorfromClass "/Game/LKH/My/My_BP/Eat/Cook.Cook_C" (Math|Transform|MakeTransform "530.000000,250.000000,20.000000" "0, 0, 0" "0.500000,0.500000,0.500000") "Undefined" "MultiplyWithRoot" 0 0)
    (AI|AIMoveTo self (.RandomLocation (AI|Navigation|GetRandomReachablePointinRadius (Transformation|GetActorLocation) 0.0 0 0)) 0 5.0 false)))

(fn ConstructionScript)