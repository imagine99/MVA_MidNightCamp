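; BP_AI3 is an AI pawn that wanders at random until given a location to head toward.
; Serch loops AIMoveTo to random reachable points within a radius and, after each successful move, binds CustomEvent_0 to Here actors.
; That event stores the location and sets Trace, stopping new searches while Tick moves the pawn straight toward it via unswept SetActorLocation.
; BeginPlay also creates an EXP widget.
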(event Custom|Serch
  (if (not (Variables|Default|GetTrace))
    (AI|AIMoveTo self (.RandomLocation (AI|Navigation|GetRandomReachablePointinRadius (Transformation|GetActorLocation) 1e+03 0 0)) 0 1e+02 false
      (:OnSuccess
        (Utilities|FlowControl|Delay 1.0)
        (CallFunction|Serch)
        (bind _outactors (Actor|GetAllActorsOfClass "/Game/LKH/My/My_BP/Eat/Here.Here_C"))
        (EventDispatchers|BindEventtoCall _outactors (delegate Custom|CustomEvent_0))))))

(event Custom|CustomEvent_0
  (params (location :type Vector))
  (Variables|Default|SetTarget location)
  (Variables|Default|SetTrace true))

(event EventBeginPlay
  (bind _returnvalue (UserInterface|CreateWidget "/Game/LKH/My/My_BP/UI/EXP_widget.EXP_widget_C"))
  (UserInterface|Viewport|AddtoViewport _returnvalue 0)
  (Variables|Default|SetEXP_bar _returnvalue)
  (CallFunction|Serch))

(event EventTick
  (params (DeltaSeconds :type Float%20%28single-precision%29))
  (if (Variables|Default|GetTrace)
    (Variables|Default|SetP0 (Transformation|GetActorLocation))
    (bind _output_get (Variables|Default|SetDirection (Math|Vector|Normalize (- (Variables|Default|GetTarget) (Transformation|GetActorLocation)))))
    (bind _output_get_2 (Variables|Default|SetV (* _output_get (Variables|Default|GetSpeed))))
    (bind _output_get_3 (Variables|Default|SetP (+ (Variables|Default|GetP0) (* _output_get_2 DeltaSeconds))))
    (Transformation|SetActorLocation _output_get_3 false false)))

(event Input|KeyboardEvents|X
  (params (Key :type Key%20Structure :default "None")))

(fn ConstructionScript)