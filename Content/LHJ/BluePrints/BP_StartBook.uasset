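; BP_StartBook is a clickable book actor that shrinks away, then opens and spawns a character with an explosion effect.
; BeginPlay shows the mouse cursor, enables click events and caches the actor's scale.
; Clicking the mesh starts a Tick-driven timer that steps the scale down until it would go negative.
; It then swaps to the open-book mesh, restores scale and spawns BP_SpawnCharacter plus particles once.
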(event OnClicked(compMesh)
  (params (TouchedComponent :type Primitive%20Component%20Object%20Reference) (ButtonPressed :type Key%20Structure :default "None"))
  ;[1 1 1] Timer On!
  (Variables|Default|SetisClicked? true)
  (Variables|Default|SetCurrTime 0.0))

(event EventBeginPlay
  (bind _returnvalue (Game|GetPlayerController 0))
  (Variables|/Script/Engine.PlayerController|SetbShowMouseCursor _returnvalue true)
  (Variables|/Script/Engine.PlayerController|SetbEnableClickEvents _returnvalue true)
  (Variables|Default|SetCurrScale (Transformation|GetActorScale3D)))

(event Collision|EventActorBeginOverlap
  (params (OtherActor :type Actor%20Object%20Reference)))

(event EventTick
  (params (DeltaSeconds :type Float%20%28single-precision%29))
  (if (and (Variables|Default|GetisClicked?) (Variables|Default|GetSmallerEvent))
    (bind _output_get (Variables|Default|SetCurrTime (+ DeltaSeconds (Variables|Default|GetCurrTime))))
    (if (>= _output_get (Variables|Default|GetDelayTime))
      (Variables|Default|SetCurrTime 0.0)
      (bind _output_get_2 (Variables|Default|SetCurrScale (- (Variables|Default|GetCurrScale) (* (Variables|Default|GetMinusVector) 0.01))))
      (if (>= (.x _output_get_2) 0.0)
        (Transformation|SetActorScale3D (Variables|Default|GetCurrScale))
        (else
          (Variables|Default|SetSmallerEvent false))))
    (elif (not (Variables|Default|GetSmallerEvent))
      (if (not (Variables|Default|GetisSpawn?))
        (Components|StaticMesh|SetStaticMesh (Variables|Default|GetcompMesh) "/Game/LHJ/Resource/OPENBOOK.OPENBOOK")
        (Transformation|SetActorRelativeScale3D "1.000000,1.000000,1.000000")
        ;[1 1 1] Character 여기 넣으시오.
        (Game|SpawnActorfromClass "/Game/LHJ/BluePrints/BP_SpawnCharacter.BP_SpawnCharacter_C" (Math|Transform|MakeTransform (+ (Transformation|GetActorLocation) "0.000000,0.000000,100.000000") "0, 0, 0" "1.000000,1.000000,1.000000") "Undefined" "MultiplyWithRoot" 0 0)
        (Effects|SpawnEmitteratLocation "/Game/mig/InfinityBladeEffects/Effects/FX_Treasure/Resources/P_OrePile_Explosion_Success.P_OrePile_Explosion_Success" "-260.000000,0.000000,0.000000" "0, 0, 0" "5.000000,5.000000,5.000000")
        (Variables|Default|SetisSpawn? true)))))

(fn ConstructionScript)